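; Player character for a 2D side-scrolling action game, with Enhanced Input for moving along X, jumping and firing projectiles limited by shoot energy.
; Enemy capsule overlaps apply damage, which updates the HUD health and triggers knockback, stun animation and temporary invincibility with sprite flicker, using retriggerable delays.
; On defeat from the vitality component, it detaches the camera, fades out, has GM_Action respawn the player and destroys itself.
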(event `self.ReceiveBeginPlay`
  (`parent.ReceiveBeginPlay`)
  (`|ExecutionSequence`
    (:`then_0`
      (bind _asgm_action (cast `/Game/Blueprints/GM_Action` (`GameplayStatics.GetGameMode`)))
      (set `self.GMAction` _asgm_action)
      (bind _asplayer_controller (cast `PlayerController` (`self.GetController`)))
      (`EnhancedInputSubsystemInterface.AddMappingContext` (pcsubsystem `EnhancedInputLocalPlayerSubsystem` _asplayer_controller) "/Game/input/IMC_Action.IMC_Action" 0 (struct)))
    (:`then_1`
      (set `self.BaseLateralFriction` (`CharacterMovementComponent.FallingLateralFriction` (`self.CharacterMovement`)))
      (`/Game/Widgets/WBP_Health.UpdateHealth` (`/Game/Widgets/WBP_HUD.WBP_Health` (`/Game/Blueprints/GM_Action.Hud Widget` (`self.GMAction`))) (`/Game/Blueprints/Components/BPC_Vitality.CurrentHealth` (`self.BPC_Vitality`))))
    (:`then_2`
      (add `self.Defeated` (delegate `OnDefeated`)))))

(event `EnhancedInput|/Game/input/Actions/IA_Jump`
  (params (ActionValue :type Boolean) (ElapsedSeconds :type "Float (double-precision)") (TriggeredSeconds :type "Float (double-precision)") (InputAction :type "InputAction Object Reference" :default "/Game/input/Actions/IA_Jump.IA_Jump"))
  (:`Started`
    (`self.Jump`)
    (`GameplayStatics.PlaySound2D` "/Game/Sounds/SFX/Jump_Player_Cue.Jump_Player_Cue" 1.0 1.0 0.0 null null))
  (:`Canceled`
    (`self.StopJumping` :!label _label))
  (:`Completed`
    (goto _label)))

(event `OnDefeated`
  (`PrimitiveComponent.SetCollisionEnabled` (`self.CapsuleComponent`) "NoCollision")
  (`SceneComponent.K2_DetachFromComponent` (`self.SpringArm`) "KeepWorld" "KeepWorld" "KeepWorld" true)
  (`PlayerCameraManager.StartCameraFade` :`self` (`GameplayStatics.GetPlayerCameraManager` 0) :`ToAlpha` 1.0 :`Duration` (`self.RespawnDelay`) :`bHoldWhenFinished` true)
  (`KismetSystemLibrary.Delay` (`self.RespawnDelay`))
  (`/Game/Blueprints/GM_Action.RespawnPlayer` (`self.GMAction`))
  (`PlayerCameraManager.StartCameraFade` :`self` (`GameplayStatics.GetPlayerCameraManager` 0) :`FromAlpha` 1.0 :`Duration` (`self.RespawnDelay`) :`bHoldWhenFinished` true)
  (`self.K2_DestroyActor`))

(event `EnhancedInput|/Game/input/Actions/IA_Move`
  (params (ActionValue :type "Float (double-precision)") (ElapsedSeconds :type "Float (double-precision)") (TriggeredSeconds :type "Float (double-precision)") (InputAction :type "InputAction Object Reference" :default "/Game/input/Actions/IA_Move.IA_Move"))
  (:`Triggered`
    (if (not (`self.isStunned`))
      (`self.AddMovementInput` (1.0 0.0 0.0) ActionValue)
      (`self.UpdateRotation` ActionValue))))

(event `EnhancedInput|/Game/input/Actions/IA_Shoot`
  (params (ActionValue :type Boolean) (ElapsedSeconds :type "Float (double-precision)") (TriggeredSeconds :type "Float (double-precision)") (InputAction :type "InputAction Object Reference" :default "/Game/input/Actions/IA_Shoot.IA_Shoot"))
  (bind _shootposition (`self.ShootPosition`))
  (:`Started`
    (if (not (`self.isStunned`))
      (if (> (`self.shootEnergy`) 0)
        (`/Engine/EditorBlueprintResources/StandardMacros.DecrementInt` (`self.shootEnergy`)
          (:`  `
            (set `self.isShooting` true)
            (`|SpawnActorFromClass` "/Game/Blueprints/Projectiles/Player/BP_PlayerProjectile_Regular.BP_PlayerProjectile_Regular_C" (`KismetMathLibrary.MakeTransform` (`SceneComponent.K2_GetComponentLocation` _shootposition) (`SceneComponent.K2_GetComponentRotation` _shootposition)) "AlwaysSpawn" "MultiplyWithRoot" self self)
            (`GameplayStatics.PlaySound2D` "/Game/Sounds/SFX/Shot_Regular_Cue.Shot_Regular_Cue" 1.0 1.0 0.0 null null)
            (`KismetSystemLibrary.RetriggerableDelay` (`self.ShootAnimationDuration`))
            (set `self.isShooting` false)))))))

(event `self.CapsuleComponent.OnComponentBeginOverlap`
  (params (OverlappedComponent :type "PrimitiveComponent Object Reference") (OtherActor :type "Actor Object Reference") (OtherComp :type "PrimitiveComponent Object Reference") (OtherBodyIndex :type Integer) (bFromSweep :type Boolean) (SweepResult :type "HitResult Structure (by ref)"))
  (bind _asbp_enemy_template (cast `/Game/Blueprints/characters/enemies/BP_Enemy_TEMPLATE` OtherActor))
  (if (== (`Character.CapsuleComponent` _asbp_enemy_template) OtherComp)
    (`GameplayStatics.ApplyDamage` self (`self.OverlapDamage`) null _asbp_enemy_template)))

(event `TriggerInvincibility`
  (`PrimitiveComponent.SetCollisionResponseToChannel` (`self.CapsuleComponent`) "ECC_Pawn" "ECR_Ignore")
  (bind _returnvalue (`KismetSystemLibrary.K2_SetTimerDelegate` (`|CreateDelegate` :!event `ToggleSpriteFlicker`) (`self.SpriteFlickerInterval`)))
  (set `self.FlickerHandle` _returnvalue)
  (`KismetSystemLibrary.RetriggerableDelay` (`self.InvincibilityDuration`))
  (`KismetSystemLibrary.K2_ClearAndInvalidateTimerHandle` (`self.FlickerHandle`))
  (`PrimitiveComponent.SetCollisionResponseToChannel` (`self.CapsuleComponent`) "ECC_Pawn" "ECR_Overlap")
  (`SceneComponent.SetVisibility` (`self.Sprite`) true false))

(event `self.ReceiveAnyDamage`
  (params (Damage :type "Float (single-precision)") (DamageType :type "DamageType Object Reference") (InstigatedBy :type "Controller Object Reference") (DamageCauser :type "Actor Object Reference"))
  (bind _returnvalue_x (`KismetMathLibrary.BreakVector` (`KismetMathLibrary.GetForwardVector` (`KismetMathLibrary.FindLookAtRotation` (`self.K2_GetActorLocation`) (`self.K2_GetActorLocation` DamageCauser)))))
  (`parent.ReceiveAnyDamage` Damage DamageType InstigatedBy DamageCauser)
  (`/Game/Widgets/WBP_Health.UpdateHealth` (`/Game/Widgets/WBP_HUD.WBP_Health` (`/Game/Blueprints/GM_Action.Hud Widget` (`self.GMAction`))) (`/Game/Blueprints/Components/BPC_Vitality.CurrentHealth` (`self.BPC_Vitality`)))
  (if (not (`/Game/Blueprints/Components/BPC_Vitality.isDefeated` (`self.BPC_Vitality`)))
    (`self.TriggerInvincibility`)
    (`GameplayStatics.PlaySound2D` "/Game/Sounds/SFX/Player_Hit_Cue.Player_Hit_Cue" 1.0 1.0 0.0 null null)
    (else
      (`GameplayStatics.PlaySound2D` "/Game/Sounds/SFX/Player_Defeat_Cue.Player_Defeat_Cue" 1.0 1.0 0.0 null null)))
  (set `CharacterMovementComponent.FallingLateralFriction` 0.0 (`self.CharacterMovement`))
  (`self.LaunchCharacter` (`KismetMathLibrary.MakeVector` (* (`KismetMathLibrary.SelectFloat` -1.0 1.0 (> _returnvalue_x 0.0)) (`self.KnockbackPowerHorizontal`)) (`self.KnockbackPowerVert`)) true true)
  (`PaperZDAnimInstance.JumpToNode` (`PaperZDAnimationComponent.AnimInstance` (`self.AnimationComponent`)) "JumpStun" "None")
  (set `self.isStunned` true)
  (`|ExecutionSequence`
    (:`then_0`
      (`KismetSystemLibrary.RetriggerableDelay` (`self.InvincibilityDuration`))
      (set `CharacterMovementComponent.FallingLateralFriction` (`self.BaseLateralFriction`) (`self.CharacterMovement`)))
    (:`then_1`
      (`KismetSystemLibrary.RetriggerableDelay` (`self.Stun Duration`))
      (set `self.isStunned` false))))

(event `self.OnLanded`
  (params (Hit :type "HitResult Structure (by ref)"))
  (`GameplayStatics.PlaySound2D` "/Game/Sounds/SFX/Land_Player_Cue.Land_Player_Cue" 1.0 1.0 0.0 null null))

(fn `RestoreShootEnergy`
  (`/Engine/EditorBlueprintResources/StandardMacros.IncrementInt` (`self.shootEnergy`)))

(fn `ToggleSpriteFlicker`
  (`SceneComponent.SetVisibility` (`self.Sprite`) (not (`SceneComponent.bVisible` (`self.Sprite`))) true))

(fn `UpdateRotation`
  (params (Direction :type "Float (double-precision)"))
  (`Controller.SetControlRotation` (`self.GetController`) (select `bool` (>= Direction 0.0) :`false` (`KismetMathLibrary.MakeRotator` 0.0 0.0 180.0) :`true` (`KismetMathLibrary.MakeRotator` 0.0))))

(fn `UserConstructionScript`
  (`parent.UserConstructionScript`))